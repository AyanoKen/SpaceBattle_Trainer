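; Shotgun weapon Blueprint whose WeaponTrace event fires a spread of pellets as small sphere traces from the player camera, randomized within a WeaponSpread cone.
; Each trace sends the current Points value to actors implementing BPI_Damage, or triggers any BP_SpawnButton it hits.
; Points grows after a shot that hits a damageable actor and resets after one that hits none, forming a consecutive-hit streak.
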(event `self.WeaponTrace`
  (bind _transformcomponent (`PlayerCameraManager.TransformComponent` (`GameplayStatics.GetPlayerCameraManager` 0)))
  (bind _returnvalue (`SceneComponent.K2_GetComponentLocation` _transformcomponent))
  (set `self.IsHit` false)
  (for _ (range (+ (`self.BulletCount`) 1))
    (bind _outhit (`KismetSystemLibrary.SphereTraceSingle` _returnvalue (+ (* (`KismetMathLibrary.RandomUnitVectorInConeInDegrees` (`SceneComponent.GetForwardVector` _transformcomponent) (`self.WeaponSpread`)) 8000.0) _returnvalue) 1.0 "TraceTypeQuery1"))
    (bind (_bblockinghit _binitialoverlap _time _distance _location _impactpoint _normal _impactnormal _physmat _hitactor) (`GameplayStatics.BreakHitResult` _outhit))
    (if (`KismetSystemLibrary.DoesImplementInterface` _hitactor "/Game/Blueprints/Weapons/BPI_Damage.BPI_Damage_C")
      (message `/Game/Blueprints/Weapons/BPI_Damage.TakeDamage` _hitactor (`self.Points`))
      (set `self.IsHit` true)
      (elif (`KismetMathLibrary.ClassIsChildOf` (`GameplayStatics.GetObjectClass` _hitactor) "/Game/Blueprints/BP_SpawnButton.BP_SpawnButton_C")
        (bind _asbp_spawn_button (cast `/Game/Blueprints/BP_SpawnButton` _hitactor))
        (`/Game/Blueprints/BP_SpawnButton.HitSpawnButton` _asbp_spawn_button))))
  (if (`self.IsHit`)
    (set `self.Points` (+ (`self.Points`) 100))
    (else
      (set `self.Points` 100))))

(fn `UserConstructionScript`
  (`parent.UserConstructionScript`))