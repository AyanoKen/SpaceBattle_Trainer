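; BP_Weapon is a weapon Blueprint that handles ammo, timed reloading and firing effects.
; FireWeapon compares Ammo to zero to either trigger a reload or spend a round and spawn a particle and sound at the Arrow component.
; ReloadWeapon shows a WB_WeaponReloadBar widget for ReloadTime, then refills Ammo after a Delay.
; WeaponTrace is an empty event, and BeginPlay only assigns MaxAmmo to itself, leaving Ammo untouched.
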(event `self.ReceiveBeginPlay`
  (set `self.MaxAmmo` (`self.MaxAmmo`)))

(event `ReloadWeapon`
  (bind _returnvalue (`|CreateWidget` "/Game/Blueprints/Weapons/WB_WeaponReloadBar.WB_WeaponReloadBar_C"))
  (`/Game/Blueprints/Weapons/WB_WeaponReloadBar.Reload` _returnvalue (`self.ReloadTime`))
  (`UserWidget.AddToViewport` _returnvalue 0)
  (`KismetSystemLibrary.Delay` (`self.ReloadTime`))
  (set `self.Ammo` (`self.MaxAmmo`)))

(event `FireWeapon`
  (`/Game/Blueprints/Libraries/BPML_Comparisions.INT <= INT` (`self.Ammo`)
    (:`True`
      (`self.ReloadWeapon`))
    (:`False`
      (set `self.Ammo` (- (`self.Ammo`) 1))
      (`self.WeaponFireEffects`))))

(event `WeaponTrace`)

(fn `UserConstructionScript`)

(fn `WeaponFireEffects`
  (bind (_returnvalue_location _returnvalue_rotation) (`KismetMathLibrary.BreakTransform` (`SceneComponent.K2_GetComponentToWorld` (`self.Arrow`))))
  (`GameplayStatics.SpawnEmitterAtLocation` (`self.WeaponFireEmitter`) _returnvalue_location _returnvalue_rotation (`self.WeaponFireEmitterScale`))
  (`GameplayStatics.SpawnSoundAtLocation` (`self.WeaponSound`) _returnvalue_location (struct) 1.0 1.0 0.0 null null)
  (return))