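; Spawner actor that periodically drops BP_RandoBall targets at random points inside a box volume.
; On BeginPlay a looping one-second timer calls SpawnTarget, which picks a random point within the SpawnArea box and spawns a ball there, adjusting for collisions but always spawning.
; The construction script sizes SpawnArea from the BoxExtent variable.
; An unconnected five-or-six-iteration burst-spawn loop remains in the graph but never runs.
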(event `self.ReceiveBeginPlay`
  (`KismetSystemLibrary.K2_SetTimerDelegate` (delegate `SpawnTarget`) 1.0 true))

(event `SpawnTarget`
  (bind _spawn_area (`self.Spawn_Area`))
  (bind _output_get (set `self.SpawnLocation` (`KismetMathLibrary.RandomPointInBoundingBox` (`SceneComponent.K2_GetComponentLocation` _spawn_area) (`BoxComponent.GetScaledBoxExtent` _spawn_area))))
  (`|SpawnActorFromClass` "/Game/Blueprints/BP_RandoBall.BP_RandoBall_C" (`KismetMathLibrary.MakeTransform` _output_get) "AdjustIfPossibleButAlwaysSpawn" "MultiplyWithRoot" null null))

(fn `UserConstructionScript`
  (`BoxComponent.SetBoxExtent` (`self.Spawn_Area`) (`self.BoxExtent`) true))